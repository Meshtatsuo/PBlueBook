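; Player gear radio that produces static from a sound wave through a granular synth and can be switched on or off.
; BeginPlay configures and starts the synth in scrub mode, while PlayRadio uses ToggleRadio to send note on or off.
; Tick sets a random playhead position, then immediately sets it to StormPlayheadTime.
; ChangeBroadcastFrequency only stores a random frequency, and the modular synth setup is an unused stub.
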(event Custom|PlayRadio
  (bind _radioon (Variables|Default|GetradioOn))
  (bind _wasradioon (Variables|Default|GetwasRadioOn))
  (bind _returnvalue (Math|Boolean|Equal(Boolean) _radioon _wasradioon))
  (if _radioon
    (if (not _returnvalue)
      (CallFunction|ToggleRadio true)
      (Development|PrintString "Hello"))
    (elif _returnvalue
      (CallFunction|ToggleRadio false))))

(event Custom|ChangeBroadcastFrequency
  (bind _broadcastfrequencies (Variables|Default|GetBroadcastFrequencies))
  (Variables|Default|SetCurrentBroadcastFreq (Utilities|Array|Get(acopy) _broadcastfrequencies (Math|Random|RandomIntegerinRange 0 (- (Utilities|Array|Length _broadcastfrequencies) 1)))))

(event EventBeginPlay
  (bind _static_granular (Variables|Default|GetStatic_Granular))
  (bind _successful (CallFunction|InitializeGranular))
  (if _successful
    (Class|GranularSynth|SetPlayheadTime _static_granular 3.0 3.0 "FromBeginning")
    (CameraShake|Start _static_granular)
    (Class|GranularSynth|Noteon (Variables|Default|GetStatic_Granular) 0.0 1 -1.0)
    (Variables|Default|SetradioOn true)
    (else
      (Development|PrintString "ERROR: GRANLULAR INITIALIZATION FAILED" false))))

(event EventTick
  (params (DeltaSeconds :type Float%20%28single-precision%29))
  (bind _static_granular (Variables|Default|GetStatic_Granular))
  (bind _soundwavelength (CallFunction|GetGranularSoundwaveLength))
  (Class|GranularSynth|SetPlayheadTime _static_granular (Math|Float|Clamp(Float) (Math|Random|RandomFloatinRange (- (Variables|Default|GetPlaybackRange) (/ (Variables|Default|GetPlaybackRange) 2.0)) (Variables|Default|GetPlaybackRange)) 0.01 (- _soundwavelength 0.1)) 1.0 "FromCurrentPosition")
  (Class|GranularSynth|SetPlayheadTime _static_granular (Variables|Default|GetStormPlayheadTime) 1.0 "FromBeginning"))

(fn ConstructionScript)

(fn InitializeGranular
  (bind _static_granular (Variables|Default|GetStatic_Granular))
  (bind _gstaticaudio (Variables|GranularSynthParams|GetGStaticAudio))
  (Utilities|IsValid _gstaticaudio
    (:Is%20Valid
      (Class|GranularSynth|SetSoundWave _static_granular _gstaticaudio)
      (Class|GranularSynth|SetAttackTime _static_granular (Variables|GranularSynthParams|GetGAttackTime))
      (Class|GranularSynth|SetDecayTime _static_granular (Variables|GranularSynthParams|GetGDecayTime))
      (Class|GranularSynth|SetSustainGain _static_granular (Variables|GranularSynthParams|GetGSustainGain))
      (Class|GranularSynth|SetReleaseTimeMsec _static_granular (Variables|GranularSynthParams|GetGReleaseTime))
      (Class|GranularSynth|SetGrainProbability _static_granular (Variables|GranularSynthParams|GetGGrainProbability))
      (Class|GranularSynth|SetGrainsPerSecond _static_granular (Variables|GranularSynthParams|GetGGrainsPerSec))
      (Class|GranularSynth|SetGrainVolume _static_granular (Variables|GranularSynthParams|GetGGrainVolBase) (Variables|GranularSynthParams|GetGGrainVolRange))
      (Class|GranularSynth|SetGrainDuration _static_granular (Variables|GranularSynthParams|GetGGrainBaseDuration) (Variables|GranularSynthParams|GetGGrainDurationRange))
      (Class|GranularSynth|SetGrainEnvelopeType _static_granular "Gaussian")
      (Class|GranularSynth|SetGrainPan _static_granular (Variables|GranularSynthParams|GetGGrainPanBase) (Variables|GranularSynthParams|GetGGrainPitchRange))
      (Class|GranularSynth|SetGrainPitch _static_granular (Variables|GranularSynthParams|GetGGrainPitchBase) (Variables|GranularSynthParams|GetGGrainPitchRange))
      (Class|GranularSynth|SetPlaybackSpeed _static_granular (Variables|GranularSynthParams|GetGPlaybackSpeed))
      (Class|GranularSynth|SetPlayheadTime _static_granular (Variables|GranularSynthParams|GetGPlayheadPosition) (Variables|GranularSynthParams|GetGPlayheadLerpTime) "FromBeginning")
      (Class|GranularSynth|SetScrubMode _static_granular true)
      (return true))))

(fn InitializeModular
  (return true))

(fn GetGranularSoundwaveLength
  (bind _gstaticaudio (Variables|GranularSynthParams|GetGStaticAudio))
  (Utilities|IsValid _gstaticaudio
    (:Is%20Valid
      (return (Variables|/Script/Engine.SoundBase|GetDuration _gstaticaudio)))))

(fn ToggleRadio
  (params (turnOn :type Boolean))
  (bind _static_granular (Variables|Default|GetStatic_Granular))
  (if turnOn
    (Class|GranularSynth|Noteon _static_granular 0.0 0 -1.0)
    (Variables|Default|SetradioOn true)
    (else
      (Class|GranularSynth|NoteOff _static_granular 0.0 false)
      (Variables|Default|SetradioOn false)))
  (return true))
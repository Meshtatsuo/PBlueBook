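; EMP enemy AI that roams between level TargetPoints, sometimes teleporting on arrival with particle and AnimBP cues.
; GameManager aggression sets a player-distance band for target picking, but the returned point is re-randomized, so the band isn't enforced.
; Heard noises redirect movement, while a timer switches walk/run speed and Tick plays delayed looping audio cues.
; Sight handling is disconnected, leaving the chase unreachable and its attack a print stub.
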(event OnSeePawn(PawnSensing)
  (params (Pawn :type Pawn%20Object%20Reference))
  ;[1 1 1] PawnSensing
)

(event OnHearNoise(PawnSensing)
  (params (Instigator :type Pawn%20Object%20Reference) (Location :type Vector%20%28by%20ref%29 :default "0, 0, 0") (Volume :type Float%20%28single-precision%29))
  ;[1 1 1] PawnSensing
  (AI|AIMoveTo self Location 0 5.0 false
    (:OnSuccess
      (CallFunction|Roam))))

(event Custom|Roam
  ;[1 1 1] ROAMING
  (Variables|Default|Setwalking true)
  (bind _asgame_manager (Utilities|Casting|CastToGameManager (Game|GetGameInstance)))
  (bind _targetloc (CallFunction|DetermineNextTargetLoc (Variables|/Game/GM/GameManager.GameManager_C|GetAggressionVal _asgame_manager)))
  (AI|AIMoveTo self _targetloc 0 5.0 false
    (:OnSuccess
      (bind _cantp (CallFunction|TeleportRoll))
      (if _cantp
        (bind _targetloc_2 (CallFunction|DetermineNextTargetLoc (Variables|/Game/GM/GameManager.GameManager_C|GetAggressionVal _asgame_manager)))
        (Utilities|FlowControl|Delay 1.5)
        (CallFunction|Teleport _targetloc_2)
        (Utilities|FlowControl|Delay 1.0)
        (bind _asemp_anim_bp (Utilities|Casting|CastToEmpAnimBP (Components|SkeletalMesh|GetAnimInstance (Variables|Character|GetMesh))))
        (Variables|/Game/Enemies/EMP_Enemy/Anims/EmpAnimBP.EmpAnimBP_C|SetisTeleporting _asemp_anim_bp false)
        (Variables|/Game/Enemies/EMP_Enemy/Anims/EmpAnimBP.EmpAnimBP_C|SettpOver _asemp_anim_bp true)
        (CallFunction|Roam)
        (else
          (CallFunction|Roam))))))

(event Custom|ChasePlayer
  (bind _returnvalue (Game|GetPlayerCharacter 0))
  ;[1 1 1] ChasingPlayer
  (Variables|Default|Setwalking false)
  (AI|AIMoveTo self "0, 0, 0" _returnvalue 5.0 false
    (:OnSuccess
      (if (<= (Transformation|GetDistanceTo _returnvalue) (Variables|Default|GetattackDistance))
        (CallFunction|AttackPlayer)
        (elif (Variables|Default|GetplayerIsVisible)
          (CallFunction|ChasePlayer))))))

(event Custom|UpdateMoveSpeed
  ;[1 1 1] BeginPlay, Init movespeed check
  (CallFunction|UpdateMovementSpeed))

(event Custom|AttackPlayer
  (Development|PrintString "You dead son."))

(event EventBeginPlay
  ;[1 1 1] BeginPlay, Init movespeed check
  (bind _outactors (Actor|GetAllActorsOfClass "/Script/Engine.TargetPoint"))
  (Variables|Default|SetPotentialLocs _outactors)
  (Variables|Default|Settest%20location (Transformation|GetActorLocation))
  (Utilities|Time|SetTimerbyEvent (delegate Custom|UpdateMoveSpeed) 0.033333 true)
  (CallFunction|Roam))

(event EventTick
  (params (DeltaSeconds :type Float%20%28single-precision%29))
  (Utilities|FlowControl|Delay 1e+01)
  (Audio|SpawnSoundAttached "/Game/Audio/AudioFiles/Enemies/untitled_Cue.untitled_Cue" (Variables|Default|GetAudio) "None" "0, 0, 0" "0, 0, 0" "KeepRelativeOffset" false 1.0 1.0 0.0 0 0))

(fn ConstructionScript)

(fn UpdateMovementSpeed
  (bind _charactermovement (Variables|Character|GetCharacterMovement))
  (if (Variables|Default|Getwalking)
    (Variables|/Script/Engine.CharacterMovementComponent|SetMaxWalkSpeed _charactermovement (Variables|Default|GetWalkSpeed))
    (else
      (Variables|/Script/Engine.CharacterMovementComponent|SetMaxWalkSpeed _charactermovement (Variables|Default|GetRunSpeed)))))

(fn TeleportRoll
  (if (<= (Math|Random|RandomFloatinRange 0.0 1.0) (Variables|Default|GetTPChance))
    (return true)
    (else
      (return false))))

(fn FindTPLoc
  (bind _potentiallocs (Variables|Default|GetPotentialLocs))
  (Variables|Default|SetTPLoc (Transformation|GetActorLocation (Utilities|Array|Get(acopy) _potentiallocs (Math|Random|RandomIntegerinRange 0 (- (Utilities|Array|Length _potentiallocs) 1)))))
  (Effects|SpawnEmitteratLocation "/Game/InfinityBladeEffects/Effects/FX_Monsters/FX_Monster_Ausar/P_AU_Trap_Target.P_AU_Trap_Target" (Variables|Default|GetTPLoc) "0, 0, 0" "2.000000,2.000000,2.000000")
  (bind _asemp_anim_bp (Utilities|Casting|CastToEmpAnimBP (Components|SkeletalMesh|GetAnimInstance (Variables|Character|GetMesh))))
  (Variables|/Game/Enemies/EMP_Enemy/Anims/EmpAnimBP.EmpAnimBP_C|SettpOver _asemp_anim_bp false)
  (Variables|/Game/Enemies/EMP_Enemy/Anims/EmpAnimBP.EmpAnimBP_C|SetisTeleporting _asemp_anim_bp true)
  (return))

(fn Teleport
  (params (TPLoc :type Vector))
  (Effects|SpawnEmitteratLocation "/Game/InfinityBladeEffects/Effects/FX_Ability/Summon/P_Summon_Child_Startup_large.P_Summon_Child_Startup_large" (Transformation|GetActorLocation))
  (bind _returnvalue (Transformation|Teleport TPLoc "0, 0, 0"))
  (if _returnvalue
    (Effects|SpawnEmitteratLocation "/Game/InfinityBladeEffects/Effects/FX_Monsters/FX_Monster_Ausar/P_AU_Trap_Impact.P_AU_Trap_Impact" (Transformation|GetWorldLocation (Variables|Default|GetTP_Arrive)) "0, 0, 0" "2.000000,2.000000,2.000000")
    (Effects|SpawnEmitteratLocation "/Game/InfinityBladeEffects/Effects/FX_Monsters/FX_Monster_Sentinel/P_Sentinel_LeapSlam_Impact.P_Sentinel_LeapSlam_Impact" (Transformation|GetWorldLocation (Variables|Default|GetTP_ArriveBurst)) "0, 0, 0" "2.000000,2.000000,2.000000")
    (return)
    (else
      (return))))

(fn DetermineNextTargetLoc
  (params (AggressionVal :type Float%20%28single-precision%29))
  (bind _potentiallocs (Variables|Default|GetPotentialLocs))
  (bind _potentiallocs_2 (Variables|Default|GetPotentialLocs))
  (bind _returnvalue (Utilities|Array|Length _potentiallocs))
  (bind _returnvalue_2 (- _returnvalue 1))
  (bind _returnvalue_3 (Math|Random|RandomIntegerinRange 0 _returnvalue_2))
  (bind _output (Utilities|Array|Get(acopy) _potentiallocs_2 _returnvalue_3))
  (if (Math|Float|InRange(Float) AggressionVal 0.0 2e+01)
    (LocalVariables|SetmaxRangeToPlayer 5e+03)
    (LocalVariables|SetminRangeToPlayer 3.5e+03)
    (while (LocalVariables|GetneedsTarget) :!label _label
      (if (Math|Float|InRange(Float) (Transformation|GetDistanceTo _output (Game|GetPlayerController 0)) (LocalVariables|GetminRangeToPlayer) (LocalVariables|GetmaxRangeToPlayer))
        (LocalVariables|SetneedsTarget false)))
    (return (Transformation|GetActorLocation _output))
    (elif (Math|Float|InRange(Float) AggressionVal 20.00001 49.999901)
      (LocalVariables|SetmaxRangeToPlayer 7e+03)
      (LocalVariables|SetminRangeToPlayer 5e+03)
      (goto _label)
      (elif (Math|Float|InRange(Float) AggressionVal 5e+01 74.999901)
        (LocalVariables|SetmaxRangeToPlayer 9e+03)
        (LocalVariables|SetminRangeToPlayer 6.2e+03)
        (goto _label)
        (elif (Math|Float|InRange(Float) AggressionVal 75.0 1e+02)
          (LocalVariables|SetmaxRangeToPlayer 1.5e+04)
          (LocalVariables|SetminRangeToPlayer 8e+03)
          (goto _label))))))